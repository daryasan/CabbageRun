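; BP_Buff is a health pickup actor that restores one point of health to the player character, up to a cap.
; It starts hidden, and ShowBuff and HideBuff toggle its mesh visibility, sphere collision and enabled flag.
; When the player overlaps the sphere while enabled and below maximum health, it heals, refreshes the health UI, then hides its mesh and disables collision.
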(event `self.ReceiveBeginPlay`
  (`self.Hide Buff`))

(event `self.Sphere.OnComponentBeginOverlap`
  (params (OverlappedComponent :type "PrimitiveComponent Object Reference") (OtherActor :type "Actor Object Reference") (OtherComp :type "PrimitiveComponent Object Reference") (OtherBodyIndex :type Integer) (bFromSweep :type Boolean) (SweepResult :type "HitResult Structure (by ref)"))
  (bind _returnvalue (`GameplayStatics.GetPlayerCharacter` 0))
  (if (`self.Is Enabled`)
    (if (== OtherActor _returnvalue)
      (bind _asbp_third_person_character (cast `/Game/ThirdPerson/Blueprints/BP_ThirdPersonCharacter` _returnvalue))
      (bind _health (`/Game/ThirdPerson/Blueprints/BP_ThirdPersonCharacter.Health` _asbp_third_person_character))
      (if (< _health 5)
        (set `/Game/ThirdPerson/Blueprints/BP_ThirdPersonCharacter.Health` (+ 1 _health) _asbp_third_person_character)
        (`/Game/ThirdPerson/Blueprints/BP_ThirdPersonCharacter.UpdateHealthUI` _asbp_third_person_character)
        (`SceneComponent.SetVisibility` (`self.StaticMesh`) false false)
        (`PrimitiveComponent.SetCollisionEnabled` (`self.Sphere`) "NoCollision")))))

(event `Show Buff`
  (`SceneComponent.SetVisibility` (`self.StaticMesh`) true false)
  (`PrimitiveComponent.SetCollisionEnabled` (`self.Sphere`) "QueryAndPhysics")
  (set `self.Is Enabled` true))

(event `Hide Buff`
  (`SceneComponent.SetVisibility` (`self.StaticMesh`) false false)
  (`PrimitiveComponent.SetCollisionEnabled` (`self.Sphere`) "NoCollision")
  (set `self.Is Enabled` false))

(fn `UserConstructionScript`)
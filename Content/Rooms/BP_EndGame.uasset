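; BP_EndGame is a level-end trigger actor that lets the player win when the third-person character touches it.
; It starts hidden, with its End component and text invisible and its sphere collision disabled.
; A MakeVisible event shows both and turns the sphere collision on.
; Overlapping the sphere then calls Win on the BP_ThirdPersonCharacter.
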(event `MakeVisible`
  (`SceneComponent.SetVisibility` (`self.End`) true false)
  (`PrimitiveComponent.SetCollisionEnabled` (`self.Sphere`) "QueryAndPhysics")
  (`SceneComponent.SetVisibility` (`self.TextRender`) true false))

(event `self.ReceiveBeginPlay`
  (`SceneComponent.SetVisibility` (`self.End`) false false)
  (`PrimitiveComponent.SetCollisionEnabled` (`self.Sphere`) "NoCollision")
  (`SceneComponent.SetVisibility` (`self.TextRender`) false false))

(event `self.Sphere.OnComponentBeginOverlap`
  (params (OverlappedComponent :type "PrimitiveComponent Object Reference") (OtherActor :type "Actor Object Reference") (OtherComp :type "PrimitiveComponent Object Reference") (OtherBodyIndex :type Integer) (bFromSweep :type Boolean) (SweepResult :type "HitResult Structure (by ref)"))
  (bind _asbp_third_person_character (cast `/Game/ThirdPerson/Blueprints/BP_ThirdPersonCharacter` OtherActor))
  (if (`KismetSystemLibrary.IsValid` _asbp_third_person_character)
    (`/Game/ThirdPerson/Blueprints/BP_ThirdPersonCharacter.Win` _asbp_third_person_character)))

(fn `UserConstructionScript`)
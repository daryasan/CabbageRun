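; Moving trap Blueprint for rooms that slides its Collision component back and forth for as long as it is in play.
; After the parent BeginPlay, two eased MoveComponentTo calls alternate between MotionRange and its negation, looping back on completion.
; Each move's duration is MovingTime scaled by DifficultyMul, and the Blueprint itself adds no active overlap or tick logic.
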(event `self.ReceiveBeginPlay`
  (`parent.ReceiveBeginPlay`)
  (`KismetSystemLibrary.MoveComponentTo` (`self.Collision`) (`self.MotionRange`) (struct) true true (* (`self.Difficulty Mul`) (`self.MovingTime`)) :!label _label)
  (`KismetSystemLibrary.MoveComponentTo` (`self.Collision`) (* (`self.MotionRange`) (-1.0 -1.0 -1.0)) (struct) true true (* (`self.Difficulty Mul`) (`self.MovingTime`)))
  (goto _label))

(fn `UserConstructionScript`
  (`parent.UserConstructionScript`))
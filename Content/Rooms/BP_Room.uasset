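; BP_Room is a room actor that tracks level progression and triggers the switch to the end-game state.
; BeginPlay picks a random maximum level between two bounds.
; IncreaseLevel increments the counter and updates a text render.
; At the maximum, it disables every BP_TeleportDoor, hides two other texts and reveals BP_EndGame actors, finding both classes with GetAllActorsOfClass.
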(event `Set Level Text`
  (`TextRenderComponent.K2_SetText` (`self.TextRender3`) (`KismetTextLibrary.Conv_StringToText` (`KismetStringLibrary.Conv_IntToString` (`self.Level`)))))

(event `IncreaseLevel`
  (set `self.Level` (+ (`self.Level`) 1))
  (`self.Set Level Text`)
  (if (== (`self.Level`) (`self.MaxLevel`))
    (bind _outactors (`GameplayStatics.GetAllActorsOfClass` "/Game/Rooms/BP_TeleportDoor.BP_TeleportDoor_C"))
    (`/Game/Rooms/BP_TeleportDoor.DisableMyself` _outactors)
    (`SceneComponent.SetVisibility` (`self.TextRender2`) false false)
    (`SceneComponent.SetVisibility` (`self.TextRender1`) false false)
    (bind _outactors_2 (`GameplayStatics.GetAllActorsOfClass` "/Game/Rooms/BP_EndGame.BP_EndGame_C"))
    (`/Game/Rooms/BP_EndGame.MakeVisible` _outactors_2)))

(event `self.ReceiveBeginPlay`
  (set `self.MaxLevel` (`KismetMathLibrary.RandomIntegerInRange` 6 10)))

(fn `UserConstructionScript`)
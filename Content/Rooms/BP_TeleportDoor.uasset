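; BP_TeleportDoor is a room door that teleports the third-person character and advances the game's level.
; On box overlap it moves the player to RespawnPosition, transformed from the door's local space to world space.
; It then finds all traps, rooms and buffs by class to set the new difficulty, increase the level, and show or hide buffs per ShowBuff.
; DisableMyself swaps the door for a wall and turns off the trigger.
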(event `self.Box.OnComponentBeginOverlap`
  (params (OverlappedComponent :type "PrimitiveComponent Object Reference") (OtherActor :type "Actor Object Reference") (OtherComp :type "PrimitiveComponent Object Reference") (OtherBodyIndex :type Integer) (bFromSweep :type Boolean) (SweepResult :type "HitResult Structure (by ref)"))
  (bind _asbp_third_person_character (cast `/Game/ThirdPerson/Blueprints/BP_ThirdPersonCharacter` OtherActor))
  (if (`KismetSystemLibrary.IsValid` _asbp_third_person_character)
    (`self.K2_SetActorLocation` OtherActor (`KismetMathLibrary.TransformLocation` (`self.GetTransform`) (`self.Respawn Position`)) false true)
    (bind _outactors (`GameplayStatics.GetAllActorsOfClass` "/Game/Rooms/BP_Trap.BP_Trap_C"))
    (`/Game/Rooms/BP_Trap.SetDifficulty` _outactors (`self.New Difficulty`))
    (bind _outactors_2 (`GameplayStatics.GetAllActorsOfClass` "/Game/Rooms/BP_Room.BP_Room_C"))
    (`/Game/Rooms/BP_Room.IncreaseLevel` _outactors_2)
    (if (`self.Show Buff`)
      (bind _outactors_3 (`GameplayStatics.GetAllActorsOfClass` "/Game/Rooms/BP_Buff.BP_Buff_C"))
      (`/Game/Rooms/BP_Buff.Show Buff` _outactors_3)
      (else
        (bind _outactors_4 (`GameplayStatics.GetAllActorsOfClass` "/Game/Rooms/BP_Buff.BP_Buff_C"))
        (`/Game/Rooms/BP_Buff.Hide Buff` _outactors_4)))))

(event `DisableMyself`
  (`SceneComponent.SetVisibility` (`self.Door`) false false)
  (`SceneComponent.SetVisibility` (`self.Doorframe`) false false)
  (`PrimitiveComponent.SetCollisionEnabled` (`self.Box`) "NoCollision")
  (`SceneComponent.SetVisibility` (`self.Wall`) true false))

(fn `UserConstructionScript`)
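; BP_Trap is a trap actor that costs the player character one Health when it enters the Collision component.
; Begin and end overlaps toggle IsInTrap, and ApplyDamage adds a signed amount to Health, then refreshes the health UI.
; A Delay on Tick repeats ApplyDamage while IsInTrap is set, but with zero change.
; SetDifficulty subtracts from DifficultyMul, which the damage logic never reads.
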(event `self.Collision.OnComponentBeginOverlap`
  (params (OverlappedComponent :type "PrimitiveComponent Object Reference") (OtherActor :type "Actor Object Reference") (OtherComp :type "PrimitiveComponent Object Reference") (OtherBodyIndex :type Integer) (bFromSweep :type Boolean) (SweepResult :type "HitResult Structure (by ref)"))
  (if (== OtherActor (`GameplayStatics.GetPlayerCharacter` 0))
    (set `self.Is In Trap` true)
    (bind _asbp_third_person_character (cast `/Game/ThirdPerson/Blueprints/BP_ThirdPersonCharacter` OtherActor))
    (if (`KismetSystemLibrary.IsValid` _asbp_third_person_character)
      (`self.Apply Damage` _asbp_third_person_character -1))))

(event `self.Collision.OnComponentEndOverlap`
  (params (OverlappedComponent :type "PrimitiveComponent Object Reference") (OtherActor :type "Actor Object Reference") (OtherComp :type "PrimitiveComponent Object Reference") (OtherBodyIndex :type Integer))
  (set `self.Is In Trap` false))

(event `self.ReceiveTick`
  (params (DeltaSeconds :type "Float (single-precision)"))
  (`KismetSystemLibrary.Delay` (`self.Damage Interval`))
  (bind _asbp_third_person_character (cast `/Game/ThirdPerson/Blueprints/BP_ThirdPersonCharacter` (`GameplayStatics.GetPlayerCharacter` 0)))
  (if (`self.Is In Trap`)
    (`self.Apply Damage` _asbp_third_person_character)))

(event `SetDifficulty`
  (params (`New Diff` :type "Float (double-precision)"))
  (set `self.Difficulty Mul` (- (`self.Difficulty Mul`) `New Diff`)))

(fn `Apply Damage`
  (params (Player :type "/Game/ThirdPerson/Blueprints/BP_ThirdPersonCharacter Object Reference") (Health :type Integer))
  (set `/Game/ThirdPerson/Blueprints/BP_ThirdPersonCharacter.Health` (+ Health (`/Game/ThirdPerson/Blueprints/BP_ThirdPersonCharacter.Health` Player)) Player)
  (`/Game/ThirdPerson/Blueprints/BP_ThirdPersonCharacter.UpdateHealthUI` Player))

(fn `UserConstructionScript`)